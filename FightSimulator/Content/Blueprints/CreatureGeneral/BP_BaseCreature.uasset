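; BP_BaseCreature is a creature Blueprint that shows its health on an attached health bar widget.
; BeginPlay caches the component's WBP_HealthBar, and Tick sets its progress bar to CurrentHP over MaxHP every frame.
; A SetupHealthBar event rotates the widget component to face the player camera using a look-at rotation, but nothing in this file calls it.
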(event `self.SetupHealthBar`
  (bind _healthbarwidget (`self.HealthBarWidget`))
  (`SceneComponent.K2_SetWorldRotation` _healthbarwidget (`KismetMathLibrary.FindLookAtRotation` (`SceneComponent.K2_GetComponentLocation` _healthbarwidget) (`SceneComponent.K2_GetComponentLocation` (`PlayerCameraManager.TransformComponent` (`GameplayStatics.GetPlayerCameraManager` 0)))) false false))

(event `self.ReceiveBeginPlay`
  (bind _aswbp_health_bar (cast `/Game/Blueprints/UI/WBP_HealthBar` (`WidgetComponent.GetWidget` (`self.HealthBarWidget`))))
  (set `self.HealthBar` _aswbp_health_bar))

(event `self.ReceiveTick`
  (params (DeltaSeconds :type "Float (single-precision)"))
  (`ProgressBar.SetPercent` (`/Game/Blueprints/UI/WBP_HealthBar.pbHealthBar` (`self.HealthBar`)) (/ (`self._currentHP`) (`self._maxHP`))))

(fn `UserConstructionScript`)